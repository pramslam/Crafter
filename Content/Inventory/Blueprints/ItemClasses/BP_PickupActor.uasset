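; BP_PickupActor is a world pickup that gives an item stack to the player's inventory when touched.
; On sphere overlap it casts to PuzzlePlayerCharacter and calls AddItem on its inventory with the configured item class and amount.
; If only part fits, it keeps the remainder as its new amount; otherwise it destroys itself once the add succeeds.
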(event OnComponentBeginOverlap(Sphere)
  (params (OverlappedComponent :type Primitive%20Component%20Object%20Reference) (OtherActor :type Actor%20Object%20Reference) (OtherComp :type Primitive%20Component%20Object%20Reference) (OtherBodyIndex :type Integer) (bFromSweep :type Boolean) (SweepResult :type Hit%20Result%20Structure%20%28by%20ref%29))
  (bind _aspuzzle_player_character (Utilities|Casting|CastToPuzzlePlayerCharacter OtherActor))
  (Utilities|IsValid (Variables|/Game/PuzzleBP/Blueprints/PuzzlePlayerCharacter.PuzzlePlayerCharacter_C|GetInventoryRef _aspuzzle_player_character)
    (:Is%20Valid
      (bind (_success_ _rest) (Default|AddItem (Variables|/Game/PuzzleBP/Blueprints/PuzzlePlayerCharacter.PuzzlePlayerCharacter_C|GetInventoryRef _aspuzzle_player_character) (Variables|Default|GetItemToAdd) (Variables|Default|GetAmount)))
      (if _success_
        (if (> _rest 0)
          (Variables|Default|SetAmount _rest)
          (else
            (Actor|DestroyActor)))))))

(fn ConstructionScript)