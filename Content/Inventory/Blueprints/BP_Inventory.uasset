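; Slot-based inventory that stores item class and amount pairs in a fixed-size array and owns its on-screen UI.
; On BeginPlay it sizes the slots, creates the main widget and caches its inventory widget for show, hide and per-slot refreshes.
; AddItem recursively fills partial stacks up to the max size, then empty slots, placing non-stackable items one per slot and returning any leftover as Rest.
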(event Custom|UpdateSlotAtIndex
  (params (Index :type Integer))
  (Default|UpdateSlot (Utilities|Array|Get(acopy) (Variables|/Game/Inventory/Widgets/Inventory.Inventory_C|GetSlotsWidgets (Variables|Default|GetInventoryWidget)) Index)))

(event EventBeginPlay
  (Utilities|Array|Resize (Variables|Default|GetSlots) (Variables|Default|GetAmountOfSlots))
  (bind _returnvalue (UserInterface|CreateWidget "/Game/Inventory/Widgets/MainWidget.MainWidget_C" 0 self (Variables|Default|GetSlotsPerRow)))
  (bind _output_get (Variables|Default|SetMainWidget _returnvalue))
  (Variables|Default|SetInventoryWidget (Variables|/Game/Inventory/Widgets/MainWidget.MainWidget_C|GetInventoryWidget _output_get))
  (UserInterface|Viewport|AddtoViewport (Variables|Default|GetMainWidget) 0))

(fn ConstructionScript)

(fn IsSlotEmpty?
  (params (Index :type Integer))
  (return (not (Utilities|IsValidClass (.itemclass (Utilities|Array|Get(acopy) (Variables|Default|GetSlots) Index))))))

(fn GetItemInfoatIndex
  (params (Index :type Integer))
  (bind _slots (Variables|Default|GetSlots))
  (bind _item (Utilities|Array|Get(acopy) _slots Index))
  (if (Utilities|IsValidClass (.itemclass _item)) ; Check if Valid Class and returns iteminfo or empty slot
    (return false (Utilities|GetClassDefaults (.itemclass _item)) (.amount _item))
    (else
      (return true "" 0))))

(fn SearchEmptySlot
  (bind (_array_element _array_index) (Utilities|Array|ForEachLoopwithBreak (Variables|Default|GetSlots) :!label _label)
    (:LoopBody
      (if (not (Utilities|IsValidClass (.itemclass _array_element)))
        (LocalVariables|SetlocalBool true)
        (LocalVariables|SetlocalIndex _array_index)
        (goto _label Break)))
    (:Completed
      (return (LocalVariables|GetlocalBool) (LocalVariables|GetlocalIndex)))))

(fn SearchFreeStack
  (params (ItemClass :type BP%20Master%20Item%20Class%20Reference))
  (bind (_array_element _array_index) (Utilities|Array|ForEachLoopwithBreak (Variables|Default|GetSlots) :!label _label)
    (:LoopBody
      (if (Utilities|IsValidClass (.itemclass _array_element))
        (if (and (== (.itemclass _array_element) ItemClass) (< (.amount _array_element) (Variables|Default|GetMaxStackSize)))
          (LocalVariables|SetlocalBool true)
          (LocalVariables|SetlocalIndex _array_index)
          (goto _label Break))))
    (:Completed
      (return (LocalVariables|GetlocalBool) (LocalVariables|GetlocalIndex)))))

(fn AddItem
  (params (ItemClass :type BP%20Master%20Item%20Class%20Reference) (Amount :type Integer))
  (bind _output_get (LocalVariables|SetlocalClass ItemClass))
  (LocalVariables|SetlocalAmount Amount)
  (if (.canBeStacked? (Utilities|Struct|BreakS_ItemInfo (Utilities|GetClassDefaults _output_get))) ; Check if Item Can be Stacked
    (bind (_success_ _index) (CallFunction|SearchFreeStack (LocalVariables|GetlocalClass)))
    (if _success_ ; Check for Free Stack
      (LocalVariables|SetlocalFoundIndex _index)
      (if (> (+ (.amount (Utilities|Array|Get(acopy) (Variables|Default|GetSlots) (LocalVariables|GetlocalFoundIndex))) (LocalVariables|GetlocalAmount)) (Variables|Default|GetMaxStackSize)) ; Check Stack Size
        (LocalVariables|SetlocalAmount (- (+ (.amount (Utilities|Array|Get(acopy) (Variables|Default|GetSlots) (LocalVariables|GetlocalFoundIndex))) (LocalVariables|GetlocalAmount)) (Variables|Default|GetMaxStackSize)))
        (Utilities|Array|SetArrayElem (Variables|Default|GetSlots) (LocalVariables|GetlocalFoundIndex) (Utilities|Struct|MakeS_InventorySlot (LocalVariables|GetlocalClass) (Variables|Default|GetMaxStackSize)))
        (CallFunction|UpdateSlotatIndex (LocalVariables|GetlocalFoundIndex))
        (bind _rest (CallFunction|AddItem (LocalVariables|GetlocalClass) (LocalVariables|GetlocalAmount)))
        (return true _rest)
        (else
          (Utilities|Array|SetArrayElem (Variables|Default|GetSlots) (LocalVariables|GetlocalFoundIndex) (Utilities|Struct|MakeS_InventorySlot (LocalVariables|GetlocalClass) (+ (.amount (Utilities|Array|Get(acopy) (Variables|Default|GetSlots) (LocalVariables|GetlocalFoundIndex))) (LocalVariables|GetlocalAmount))))
          (CallFunction|UpdateSlotatIndex (LocalVariables|GetlocalFoundIndex))
          (return true 0)))
      (else
        (bind (_success__2 _index_2) (CallFunction|SearchEmptySlot))
        (if _success__2 ; Check for Free Slot
          (LocalVariables|SetlocalFoundIndex _index_2)
          (if (> (LocalVariables|GetlocalAmount) (Variables|Default|GetMaxStackSize))
            (Utilities|Array|SetArrayElem (Variables|Default|GetSlots) (LocalVariables|GetlocalFoundIndex) (Utilities|Struct|MakeS_InventorySlot (LocalVariables|GetlocalClass) (Variables|Default|GetMaxStackSize)))
            (CallFunction|UpdateSlotatIndex (LocalVariables|GetlocalFoundIndex))
            (bind _rest_2 (CallFunction|AddItem (LocalVariables|GetlocalClass) (- (LocalVariables|GetlocalAmount) (Variables|Default|GetMaxStackSize))))
            (return true _rest_2)
            (else
              (Utilities|Array|SetArrayElem (Variables|Default|GetSlots) (LocalVariables|GetlocalFoundIndex) (Utilities|Struct|MakeS_InventorySlot (LocalVariables|GetlocalClass) (LocalVariables|GetlocalAmount)))
              (CallFunction|UpdateSlotatIndex (LocalVariables|GetlocalFoundIndex))
              (return true 0)))
          (else
            (return false (LocalVariables|GetlocalAmount)) ; No Free Stacks, No Empty Slots
          ))))
    (else
      (bind (_success__3 _index_3) (CallFunction|SearchEmptySlot))
      (if _success__3
        (LocalVariables|SetlocalFoundIndex _index_3)
        (Utilities|Array|SetArrayElem (Variables|Default|GetSlots) (LocalVariables|GetlocalFoundIndex) (Utilities|Struct|MakeS_InventorySlot (LocalVariables|GetlocalClass) 1))
        (CallFunction|UpdateSlotatIndex (LocalVariables|GetlocalFoundIndex))
        (if (> (LocalVariables|GetlocalAmount) 1)
          (bind _rest_3 (CallFunction|AddItem (LocalVariables|GetlocalClass) (- (LocalVariables|GetlocalAmount) 1))) ; Non-Stackable Items will be added to another slot
          (return true _rest_3)
          (else
            (return true 0)))
        (else
          (return false (LocalVariables|GetlocalAmount)) ; No empty Slots, not stackable item
        )))))

(fn GetAmountatIndex
  (params (Index :type Integer))
  (return (.amount (Utilities|Array|Get(acopy) (Variables|Default|GetSlots) Index))))

(fn ShowInventory
  (Widget|SetVisibility (Variables|Default|GetInventoryWidget) "Visible")
  (Variables|Default|SetIsVisible? true)
  (Widget|SetIsEnabled (Variables|Default|GetInventoryWidget) true)
  (return))

(fn HideInventory
  (Widget|SetVisibility (Variables|Default|GetInventoryWidget) "Hidden")
  (Variables|Default|SetIsVisible? false)
  (Widget|SetIsEnabled (Variables|Default|GetInventoryWidget) false)
  (return))